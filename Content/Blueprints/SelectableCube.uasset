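; SelectableCube is a test Blueprint for mouse interaction that prints debug messages and has no selection logic.
; Its static mesh component's cursor begin-over, end-over, click and release events each print a string.
; Two custom actor-level handlers for cursor-over and click also print, but their delegate binds sit inside the handlers, with no initial bind shown.
; The construction script and NewFunction are empty.
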(event OnBeginCursorOver(StaticMeshComponent)
  (params (TouchedComponent :type Primitive%20Component%20Object%20Reference))
  (Development|PrintString "Begin Over"))

(event OnEndCursorOver(StaticMeshComponent)
  (params (TouchedComponent :type Primitive%20Component%20Object%20Reference))
  (Development|PrintString "End Over"))

(event OnClicked(StaticMeshComponent)
  (params (TouchedComponent :type Primitive%20Component%20Object%20Reference) (ButtonPressed :type Key%20Structure :default "None"))
  (Development|PrintString "Clicked"))

(event OnReleased(StaticMeshComponent)
  (params (TouchedComponent :type Primitive%20Component%20Object%20Reference) (ButtonReleased :type Key%20Structure :default "None"))
  (Development|PrintString "Released"))

(event Custom|OnBeginCursorOver_Event
  (params (TouchedActor :type Actor%20Object%20Reference))
  (EventDispatchers|BindEventtoOnBeginCursorOver (delegate Custom|OnBeginCursorOver_Event))
  (Development|PrintString "Begin Over"))

(event Custom|OnClicked_Event
  (params (TouchedActor :type Actor%20Object%20Reference) (ButtonPressed :type Key%20Structure :default "None"))
  (EventDispatchers|BindEventtoOnClicked (delegate Custom|OnClicked_Event))
  (Development|PrintString "Clicked"))

(fn ConstructionScript)

(fn NewFunction)